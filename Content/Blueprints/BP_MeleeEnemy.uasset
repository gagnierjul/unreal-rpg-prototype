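; BP_MeleeEnemy is a melee enemy with single-slash and combo attacks that damage the player.
; Attack and ComboAttack play montages whose Attack Start and Attack End notifies open and close the active hit window.
; Box overlaps with a non-immune BP_Player during that window flag success and subtract fixed HP from Player.
; A shared DoOnce, reset at Attack End, limits damage to once per window.
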(event `ComboAttack`
  (bind _player (`self.Player`))
  ;[1 1 1] Combo Attack Handler
  (bind _notifyname (`|PlayMontage` (`self.Mesh`) "/Game/Animations/MeleeEnemy/AM_MeleeEnemy_ComboSlashGood.AM_MeleeEnemy_ComboSlashGood")
    (:`OnNotifyBegin`
      (switch `name` _notifyname
        (:`AttackStart`
          (set `self.IsAttackActive` true))
        (:`AttackEnd`
          (set `self.IsAttackActive` false)
          (set `self.IsAttackSuccess` false)
          (goto _label :!via `Reset`))))))

(event `self.Box.OnComponentBeginOverlap`
  (params (OverlappedComponent :type "PrimitiveComponent Object Reference") (OtherActor :type "Actor Object Reference") (OtherComp :type "PrimitiveComponent Object Reference") (OtherBodyIndex :type Integer) (bFromSweep :type Boolean) (SweepResult :type "HitResult Structure (by ref)"))
  (bind _player (`self.Player`))
  ;[1 1 1] Mace Hit Handler
  (if (`self.IsAttackActive`)
    (bind _asbp_player (cast `/Game/Blueprints/BP_Player` OtherActor))
    (if (not (`/Game/Blueprints/BP_Player.IsImmune` _asbp_player))
      (set `self.IsAttackSuccess` true)
      (`/Engine/EditorBlueprintResources/StandardMacros.DoOnce` false :!label _label
        (:`Completed`
          (set `/Game/Blueprints/BP_Player.HP` (- (`/Game/Blueprints/BP_Player.HP` _player) 5) _player))))))

(event `Attack`
  ;[1 1 1] Attack Handler
  (bind _notifyname (`|PlayMontage` (`self.Mesh`) "/Game/Animations/MeleeEnemy/AM_MeleeEnemy_Slash.AM_MeleeEnemy_Slash")
    (:`OnNotifyBegin`
      (switch `name` _notifyname
        (:`AttackStart`
          (set `self.IsAttackActive` true))
        (:`AttackEnd`
          (set `self.IsAttackActive` false)
          (goto _label :!via `Reset`))))))

(fn `UserConstructionScript`
  (`parent.UserConstructionScript`))