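; Base enemy Blueprint, judging by its name, with a health check and an overhead-style widget that follows the camera's orientation.
; On BeginPlay it caches the player pawn and passes itself to its WBP_Enemy widget.
; Tick re-orients the widget from the camera rotation plus a 180-degree offset.
; CheckIsDead, when invoked, spawns a BP_Skull at a random nearby point and destroys the enemy if HP is depleted.
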(event `self.ReceiveBeginPlay`
  ;[1 0 0] EVENT BEGIN PLAY
  (bind _asbp_player (cast `/Game/Blueprints/BP_Player` (`GameplayStatics.GetPlayerPawn` 0)))
  (set `self.Player` _asbp_player)
  (bind _aswbp_enemy (cast `/Game/Blueprints/WBP_Enemy` (`WidgetComponent.GetUserWidgetObject` (`self.Widget`))))
  (set `/Game/Blueprints/WBP_Enemy.Enemy` self _aswbp_enemy))

(event `self.ReceiveTick`
  (params (DeltaSeconds :type "Float (single-precision)"))
  ;[1 0 0] EVENT TICK (Widget Rotation Handler)
  (`SceneComponent.K2_SetWorldRotation` (`self.Widget`) (`KismetMathLibrary.ComposeRotators` (`PlayerCameraManager.GetCameraRotation` (`GameplayStatics.GetPlayerCameraManager` 0)) (struct :`Yaw` 180.0)) false false))

(event `CheckIsDead`
  ;[1 1 1] Check is Dead
  (if (<= (`self.HP`) 0)
    (`|SpawnActorFromClass` "/Game/Blueprints/BP_Skull.BP_Skull_C" (`KismetMathLibrary.MakeTransform` (`KismetMathLibrary.RandomPointInBoundingBox` (`self.K2_GetActorLocation`) (150.0 150.0 0.0))) "Undefined" "OverrideRootScale" null null)
    (`self.K2_DestroyActor`)))

(fn `UserConstructionScript`)