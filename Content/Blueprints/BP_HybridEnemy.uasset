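; BP_HybridEnemy is an enemy that supports both melee and ranged attacks against BP_Player.
; Each tick, a short-range sphere overlap flags the player as a melee or ranged target, and low HP sets an enraged flag.
; Montage notifies open the melee damage window, where a DoOnce limits box-overlap damage to one hit per swing, and trigger projectile spawns for ranged attacks.
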(event `self.ReceiveTick`
  (params (DeltaSeconds :type "Float (single-precision)"))
  ;[1 0 0] EVENT TICK
  (`parent.ReceiveTick` DeltaSeconds)
  (`|ExecutionSequence`
    (:`then_0`
      ;[1 1 1] Range Handler (EVENT TICK)
      (bind (_outactors _returnvalue) (`KismetSystemLibrary.SphereOverlapActors` (`self.K2_GetActorLocation`) 120.0 (`|MakeArray` "ObjectTypeQuery3" :!type "EObjectTypeQuery Enum") "/Game/Blueprints/BP_Player.BP_Player_C"))
      (if _returnvalue
        (set `self.isMeleeTarget` true)
        (set `self.IsRangedTarget` false)
        (else
          (set `self.IsRangedTarget` true)
          (set `self.isMeleeTarget` false))))
    (:`then_1`
      ;[1 1 1] Enrage Handler (EVENT TICK)
      (if (<= (`self.HP`) 25)
        (set `self.IsEnraged` true)))))

(event `MeleeAttack`
  (bind _player (`self.Player`))
  ;[1 1 1] Melee Attack Handler
  (bind _notifyname (`|PlayMontage` (`self.Mesh`) "/Game/Animations/HybridEnemy/AM_HybridEnemy_Attack_Montage.AM_HybridEnemy_Attack_Montage")
    (:`OnNotifyBegin`
      (switch `name` _notifyname
        (:`AttackStart`
          (set `self.IsAttackActive` true))
        (:`AttackEnd`
          (set `self.IsAttackActive` false)
          (goto _label :!via `Reset`))))))

(event `self.Box.OnComponentBeginOverlap`
  (params (OverlappedComponent :type "PrimitiveComponent Object Reference") (OtherActor :type "Actor Object Reference") (OtherComp :type "PrimitiveComponent Object Reference") (OtherBodyIndex :type Integer) (bFromSweep :type Boolean) (SweepResult :type "HitResult Structure (by ref)"))
  (bind _player (`self.Player`))
  ;[1 1 1] Sword Hit Handler
  (cast `/Game/Blueprints/BP_Player` OtherActor)
  (if (`self.IsAttackActive`)
    (`/Engine/EditorBlueprintResources/StandardMacros.DoOnce` false :!label _label
      (:`Completed`
        (set `/Game/Blueprints/BP_Player.HP` (- (`/Game/Blueprints/BP_Player.HP` _player) 5) _player)))))

(event `RangedAttack`
  ;[1 1 1] Ranged Attack Handler
  (bind _notifyname (`|PlayMontage` (`self.Mesh`) "/Game/Animations/HybridEnemy/AM_HybridEnemy_RangedAttack.AM_HybridEnemy_RangedAttack")
    (:`OnNotifyBegin`
      (switch `name` _notifyname
        (:`AttackStart`
          (`|SpawnActorFromClass` "/Game/Blueprints/BP_EnemyProjectile.BP_EnemyProjectile_C" (`SceneComponent.K2_GetComponentToWorld` (`self.ShootFrom`)) "Undefined" "OverrideRootScale" null null))))))

(fn `UserConstructionScript`
  (`parent.UserConstructionScript`))